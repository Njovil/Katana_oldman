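; Melee enemy for a 2D side-scroller that chases and attacks the player's BP_Samurai.
; PawnSensing drives AIMoveTo or, within close X range, a cooldown-gated attack whose HitCheck damages overlapping samurai only on a specific sprite frame.
; Tick turns the enemy toward the player and updates a camera-facing health bar, hidden at zero health.
; Incoming damage reduces health and jumps the animation instance to GetHit or Death nodes.
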(event `self.ReceiveBeginPlay`
  ;[1 1 1] Получаем ссылку на объект Самурая
  (`self.GetSamuraiData`))

(event `self.ReceiveTick`
  (params (DeltaSeconds :type "Float (single-precision)"))
  ;[1 1 1] Расчёт хп и направления
  (`self.CalculateHealth`)
  (if (not (`self.EnemyIsDead`))
    (`KismetSystemLibrary.Delay` 0.2)
    (`self.GetPlayerDirection`)
    (`self.Rotate to Player`)))

(event `self.PawnSensing.OnSeePawn`
  (params (Pawn :type "Pawn Object Reference"))
  (bind _returnvalue_x (`KismetMathLibrary.BreakVector` (`self.K2_GetActorLocation` (`self.BP Samurai reference`))))
  (bind _returnvalue_x_2 (`KismetMathLibrary.BreakVector` (`self.K2_GetActorLocation` self)))
  ;[1 1 1] Движение/Атака
  (if (or (`/Game/Blueprints/SamuraiBP/BP_Samurai.IsDead` (`self.BP Samurai reference`)) (`self.EnemyIsDead`))
    _
    (elif (<= (`KismetMathLibrary.Abs` (- _returnvalue_x _returnvalue_x_2)) 70.0)
      (set `self.CanAttack` true)
      (set `self.CanMove` false)
      (`/Engine/EditorBlueprintResources/StandardMacros.DoOnce` false :!label _label
        (:`Completed`
          (`self.HitCheck`)
          (`PaperZDAnimInstance.JumpToNode` (`PaperZDAnimationComponent.AnimInstance` (`self.AnimationComponent`)) "Attack" "None")
          (`KismetSystemLibrary.Delay` 0.7)
          (goto _label :!via `Reset`)))
      (else
        (set `self.CanAttack` false)
        (set `self.CanMove` true)
        (`|AIMoveTo` self (0.0 0.0 0.0) (`GameplayStatics.GetPlayerCharacter` 0) 50.0)))))

(event `self.ReceiveAnyDamage`
  (params (Damage :type "Float (single-precision)") (DamageType :type "DamageType Object Reference") (InstigatedBy :type "Controller Object Reference") (DamageCauser :type "Actor Object Reference"))
  ;[1 1 1] Получение урона/Смерть
  (if (not (`self.EnemyIsDead`))
    (set `self.EnemyHealth` (- (`self.EnemyHealth`) Damage))
    (if (<= (`self.EnemyHealth`) 0.0)
      (`PaperZDAnimInstance.JumpToNode` (`PaperZDAnimationComponent.AnimInstance` (`self.AnimationComponent`)) "Death" "None")
      (set `self.EnemyIsDead` true)
      (else
        (`PaperZDAnimInstance.JumpToNode` (`PaperZDAnimationComponent.AnimInstance` (`self.AnimationComponent`)) "GetHit" "None")))))

(fn `CalculateHealth`
  (bind _health_bar_widget (`self.Health Bar Widget`))
  (bind (_returnvalue_roll _returnvalue_pitch) (`KismetMathLibrary.BreakRotator` (`KismetMathLibrary.FindLookAtRotation` (`SceneComponent.K2_GetComponentLocation` _health_bar_widget) (`SceneComponent.K2_GetComponentLocation` (`PlayerCameraManager.TransformComponent` (`GameplayStatics.GetPlayerCameraManager` 0))))))
  (bind _aswbp_health_bar_enemy (cast `/Game/Blueprints/UI/WBP_HealthBar_Enemy` (`WidgetComponent.GetWidget` (`self.Health Bar Widget`))))
  (`ProgressBar.SetPercent` (`/Game/Blueprints/UI/WBP_HealthBar_Enemy.HealthBar` _aswbp_health_bar_enemy) (/ (`self.EnemyHealth`) 1500.0))
  (`SceneComponent.K2_SetWorldRotation` _health_bar_widget (`KismetMathLibrary.MakeRotator` _returnvalue_roll _returnvalue_pitch 90.0) false false)
  (if (<= (`self.EnemyHealth`) 0.0)
    (`WidgetComponent.SetTintColorAndOpacity` :`self` (`self.Health Bar Widget`))))

(fn `GetPlayerDirection`
  (bind _returnvalue_x (`KismetMathLibrary.BreakVector` (`self.K2_GetActorLocation` self)))
  (bind _returnvalue_x_2 (`KismetMathLibrary.BreakVector` (`self.K2_GetActorLocation` (`self.BP Samurai reference`))))
  (if (> _returnvalue_x_2 _returnvalue_x)
    (set `self.IsPlayerToTheRight` true)
    (else
      (set `self.IsPlayerToTheRight` false))))

(fn `GetSamuraiData`
  (bind _asbp_samurai (cast `/Game/Blueprints/SamuraiBP/BP_Samurai` (`GameplayStatics.GetPlayerCharacter` 0)))
  (set `self.BP Samurai reference` _asbp_samurai))

(fn `HitCheck`
  (for _array_element (`PrimitiveComponent.GetOverlappingActors` (`self.Hitbox`) "/Game/Blueprints/SamuraiBP/BP_Samurai.BP_Samurai_C")
    ;[1 1 1] МАГИЯ, НЕ ТРОГАТЬ
    (if (!= _array_element self)
      (if (== (`PaperFlipbookComponent.GetPlaybackPositionInFrames` (`self.Sprite`)) 8)
        (`GameplayStatics.ApplyDamage` _array_element (`self.EnemyDamage`))))))

(fn `Rotate to Player`
  (bind (_returnvalue_roll _returnvalue_pitch) (`KismetMathLibrary.BreakRotator` (`self.K2_GetActorRotation`)))
  (if (`self.IsPlayerToTheRight`)
    (`self.K2_SetActorRotation` (`KismetMathLibrary.MakeRotator` _returnvalue_roll _returnvalue_pitch))
    (else
      (`self.K2_SetActorRotation` (`KismetMathLibrary.MakeRotator` _returnvalue_roll _returnvalue_pitch 180.0)))))

(fn `UserConstructionScript`)