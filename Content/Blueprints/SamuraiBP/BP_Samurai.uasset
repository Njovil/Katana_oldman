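; Player samurai character for side-scrolling melee combat, with Enhanced Input movement along world X, jumping and a two-stage attack.
; An attack opens a brief combo window for a much stronger follow-up, then a cooldown blocks spamming.
; HitCheck damages BP_Enemy actors overlapping the hitbox, while AnyDamage reduces health and triggers hit or death animation jumps.
; Tick updates a camera-tilted, fixed-yaw health bar widget, hidden at zero health.
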(event `self.ReceiveBeginPlay`
  ;[1 1 1] Создаем инпут контекст
  (bind _asplayer_controller (cast `PlayerController` (`self.GetController`)))
  (`EnhancedInputSubsystemInterface.AddMappingContext` (pcsubsystem `EnhancedInputLocalPlayerSubsystem` _asplayer_controller) "/Game/samurai/InputSamurai/IMC_SamuraiMovement.IMC_SamuraiMovement" 0 (struct)))

(event `self.ReceiveTick`
  (params (DeltaSeconds :type "Float (single-precision)"))
  ;[1 1 1] Подсчет хп
  (`self.CalculateHealth`))

(event `EnhancedInput|/Game/samurai/InputSamurai/IA_Jump`
  (params (ActionValue :type Boolean) (ElapsedSeconds :type "Float (double-precision)") (TriggeredSeconds :type "Float (double-precision)") (InputAction :type "InputAction Object Reference" :default "/Game/samurai/InputSamurai/IA_Jump.IA_Jump"))
  ;[1 1 1] Прыжок
  (:`Started`
    (if (not (`self.IsDead`))
      (`self.Jump`)
      (`PaperZDAnimInstance.JumpToNode` (`PaperZDAnimationComponent.AnimInstance` (`self.AnimationComponent`)) "Jump" "None")))
  (:`Completed`
    (`self.StopJumping`)))

(event `EnhancedInput|/Game/samurai/InputSamurai/IA_Move`
  (params (ActionValue :type "Vector2D Structure") (ElapsedSeconds :type "Float (double-precision)") (TriggeredSeconds :type "Float (double-precision)") (InputAction :type "InputAction Object Reference" :default "/Game/samurai/InputSamurai/IA_Move.IA_Move"))
  ;[1 1 1] Бег
  (:`Triggered`
    (if (not (`self.IsDead`))
      (`self.AddMovementInput` (1.0 0.0 0.0) ActionValue_X))))

(event `EnhancedInput|/Game/samurai/InputSamurai/IA_Attack`
  (params (ActionValue :type Boolean) (ElapsedSeconds :type "Float (double-precision)") (TriggeredSeconds :type "Float (double-precision)") (InputAction :type "InputAction Object Reference" :default "/Game/samurai/InputSamurai/IA_Attack.IA_Attack"))
  ;[1 1 1] Атака
  (:`Started`
    (if (and (not (`self.IsDead`)) (`self.CanAttack?`))
      (`/Engine/EditorBlueprintResources/StandardMacros.DoOnce` false :!label _label
        (:`Completed`
          (`PaperZDAnimInstance.JumpToNode` (`PaperZDAnimationComponent.AnimInstance` (`self.AnimationComponent`)) "Attack" "None")
          (set `self.SamuraiDamage` 25.0)
          (`self.HitCheck`)
          (`KismetSystemLibrary.Delay` 0.15)
          ;;[1 1 1] Окно для комбоатаки
          (set `self.IsComboAvailable` true)
          (`KismetSystemLibrary.Delay` 0.2)
          (set `self.IsComboAvailable` false)
          ;;[1 1 1] Защита от закликивания
          (set `self.CanAttack?` false)
          (`KismetSystemLibrary.Delay` 0.7)
          (set `self.CanAttack?` true)
          (goto _label :!via `Reset`))))))

(event `EnhancedInput|/Game/samurai/InputSamurai/IA_Attack_1`
  (params (ActionValue :type Boolean) (ElapsedSeconds :type "Float (double-precision)") (TriggeredSeconds :type "Float (double-precision)") (InputAction :type "InputAction Object Reference" :default "/Game/samurai/InputSamurai/IA_Attack_1.IA_Attack_1"))
  ;[1 1 1] Комбо Аттака по условию
  (:`Started`
    (if (not (`self.IsDead`))
      (if (`self.IsComboAvailable`)
        (`KismetSystemLibrary.PrintString` "COMBO")
        (`PaperZDAnimInstance.JumpToNode` (`PaperZDAnimationComponent.AnimInstance` (`self.AnimationComponent`)) "ComboAttack" "None")
        (set `self.SamuraiDamage` 200.0)
        (`self.HitCheck`)))))

(event `self.ReceiveAnyDamage`
  (params (Damage :type "Float (single-precision)") (DamageType :type "DamageType Object Reference") (InstigatedBy :type "Controller Object Reference") (DamageCauser :type "Actor Object Reference"))
  ;[1 1 1] Получение урона/смерть
  (if (not (`self.IsDead`))
    (set `self.SamuraiHealth` (- (`self.SamuraiHealth`) Damage))
    (if (<= (`self.SamuraiHealth`) 0.0)
      (`PaperZDAnimInstance.JumpToNode` (`PaperZDAnimationComponent.AnimInstance` (`self.AnimationComponent`)) "Death" "None")
      (set `self.IsDead` true)
      (else
        (`PaperZDAnimInstance.JumpToNode` (`PaperZDAnimationComponent.AnimInstance` (`self.AnimationComponent`)) "GetHit" "None")))))

(fn `CalculateHealth`
  (bind _health_bar_widget (`self.Health Bar Widget`))
  (bind (_returnvalue_roll _returnvalue_pitch) (`KismetMathLibrary.BreakRotator` (`KismetMathLibrary.FindLookAtRotation` (`SceneComponent.K2_GetComponentLocation` _health_bar_widget) (`SceneComponent.K2_GetComponentLocation` (`Actor.RootComponent` (`GameplayStatics.GetPlayerCameraManager` 0))))))
  (bind _aswbp_health_bar_samurai (cast `/Game/Blueprints/UI/WBP_HealthBar_Samurai` (`WidgetComponent.GetWidget` (`self.Health Bar Widget`))))
  (`ProgressBar.SetPercent` (`/Game/Blueprints/UI/WBP_HealthBar_Samurai.HealthBar` _aswbp_health_bar_samurai) (/ (`self.SamuraiHealth`) 700.0))
  (`SceneComponent.K2_SetWorldRotation` _health_bar_widget (`KismetMathLibrary.MakeRotator` _returnvalue_roll _returnvalue_pitch 90.0) false false)
  (if (<= (`self.SamuraiHealth`) 0.0)
    (`WidgetComponent.SetTintColorAndOpacity` :`self` (`self.Health Bar Widget`))))

(fn `HitCheck`
  (for _array_element (`PrimitiveComponent.GetOverlappingActors` (`self.Hitbox`) "/Game/Blueprints/EnemyBP/BP_Enemy.BP_Enemy_C")
    (if (!= _array_element self)
      (`GameplayStatics.ApplyDamage` _array_element (`self.SamuraiDamage`)))))

(fn `UserConstructionScript`)